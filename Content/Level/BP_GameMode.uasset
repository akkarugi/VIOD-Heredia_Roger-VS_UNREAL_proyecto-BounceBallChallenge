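; BP_GameMode is the level's game mode, providing a RespawnPlayer event that replaces the player character.
; It destroys the current player, then spawns a new BP_Player at the LastCheckPoint's POS transform, or at a default transform if no checkpoint is valid.
; Player controller 0 then possesses the new pawn.
; Spawning always ignores collisions, and BeginPlay and Tick are unused.
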(event `RespawnPlayer`
  (`self.K2_DestroyActor` (`GameplayStatics.GetPlayerCharacter` 0))
  (bind _lastcheckpoint (`self.LastCheckPoint`)
    (:`then`
      (bind (_returnvalue_location _returnvalue_rotation) (`KismetMathLibrary.BreakTransform` (`SceneComponent.K2_GetComponentToWorld` (`/Game/Level/BP_Checkpoint.POS` _lastcheckpoint))))
      (bind _returnvalue (`|SpawnActorFromClass` "/Game/Level/BP_Player.BP_Player_C" (`KismetMathLibrary.MakeTransform` _returnvalue_location _returnvalue_rotation) "AlwaysSpawn" "MultiplyWithRoot" null null))
      (`Controller.Possess` (`GameplayStatics.GetPlayerController` 0) _returnvalue))
    (:`else`
      (bind _returnvalue_2 (`|SpawnActorFromClass` "/Game/Level/BP_Player.BP_Player_C" (`KismetMathLibrary.MakeTransform` (0.0 0.0 0.0)) "AlwaysSpawn" "MultiplyWithRoot" null null))
      (`Controller.Possess` (`GameplayStatics.GetPlayerController` 0) _returnvalue_2))))

(fn `UserConstructionScript`)