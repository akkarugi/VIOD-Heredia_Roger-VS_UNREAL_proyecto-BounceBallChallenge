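; Tutorial grapple point actor that signals when the player is in range and lets them grapple.
; Player overlap turns the GrapplePoint material green, sets the grapple flag on BP_Controller and briefly drops global time dilation for slow motion.
; The restoring Delay runs in dilated time, so the slowdown lasts about one real second.
; Leaving the overlap restores the material and clears the flag.
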(event `self.ReceiveBeginPlay`)

(event `self.ReceiveActorBeginOverlap`
  (params (OtherActor :type "Actor Object Reference"))
  (cast `/Game/Level/BP_Player` OtherActor)
  (`PrimitiveComponent.SetMaterial` (`self.GrapplePoint`) 0 "/Game/Menu/Green.Green")
  (bind _asbp_controller (cast `/Game/Level/BP_Controller` (`GameplayStatics.GetPlayerController` 0)))
  (set `/Game/Level/BP_Controller.CanGraopple?` true _asbp_controller)
  (`GameplayStatics.SetGlobalTimeDilation` 0.2)
  (`KismetSystemLibrary.Delay` 0.2)
  (`GameplayStatics.SetGlobalTimeDilation` 1.0))

(event `self.ReceiveActorEndOverlap`
  (params (OtherActor :type "Actor Object Reference"))
  (cast `/Game/Level/BP_Player` OtherActor)
  (`PrimitiveComponent.SetMaterial` (`self.GrapplePoint`) 0 "/Game/GoodSky/Blueprint/Cylinder.Cylinder")
  (bind _asbp_controller (cast `/Game/Level/BP_Controller` (`GameplayStatics.GetPlayerController` 0)))
  (set `/Game/Level/BP_Controller.CanGraopple?` false _asbp_controller))

(event `self.ReceiveTick`
  (params (DeltaSeconds :type "Float (single-precision)")))

(fn `UserConstructionScript`)