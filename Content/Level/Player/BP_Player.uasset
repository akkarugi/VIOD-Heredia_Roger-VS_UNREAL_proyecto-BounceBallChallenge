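; BP_Player is the player's ball, with on-screen timer and coin widgets and a running coin count.
; On BeginPlay it creates both widgets, stores references to them and adds them to the viewport.
; Ball hits on actors tagged GROUND set CanJump on BP_Controller, re-enabling jumping.
; SumCoins increments the coin count by one, without touching the coin widget itself.
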(event `self.ReceiveBeginPlay`
  (bind _returnvalue (`|CreateWidget` "/Game/Level/Timer/WBP_Timer.WBP_Timer_C"))
  (bind _output_get (set `self.Timer` _returnvalue))
  (`UserWidget.AddToViewport` _output_get 0)
  (bind _returnvalue_2 (`|CreateWidget` "/Game/Level/Coins/WBP_Coin.WBP_Coin_C"))
  (bind _output_get_2 (set `self.CoinWidget` _returnvalue_2))
  (`UserWidget.AddToViewport` _output_get_2 0))

(event `self.Ball.OnComponentHit`
  (params (HitComponent :type "PrimitiveComponent Object Reference") (OtherActor :type "Actor Object Reference") (OtherComp :type "PrimitiveComponent Object Reference") (NormalImpulse :type "Vector Structure") (Hit :type "HitResult Structure (by ref)"))
  ;[1 1 1] Can jump
  (if (`self.ActorHasTag` OtherActor "GROUND")
    (bind _asbp_controller (cast `/Game/Level/Player/BP_Controller` (`GameplayStatics.GetPlayerController` 0)))
    (set `/Game/Level/Player/BP_Controller.CanJump?` true _asbp_controller)))

(fn `SumCoins`
  (set `self.Coins` (+ (`self.Coins`) 1)))

(fn `UserConstructionScript`)