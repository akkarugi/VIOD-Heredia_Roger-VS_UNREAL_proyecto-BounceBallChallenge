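; BP_Win3 is a win trigger actor that opens the WBP_Win3 menu when BP_Player overlaps it.
; The overlap fires once through a DoOnce, plays an explosion sound, adds the widget to the viewport, shows the cursor and pauses the game.
; A WinMenu flag also selects a branch that closes the menu and resumes play, but nothing here resets the DoOnce to reach it again.
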(event `self.ReceiveActorBeginOverlap`
  (params (OtherActor :type "Actor Object Reference"))
  (bind _returnvalue (`GameplayStatics.GetPlayerController` 0))
  (cast `/Game/Level/BP_Player` OtherActor)
  (`/Engine/EditorBlueprintResources/StandardMacros.DoOnce` false
    (:`Completed`
      (`GameplayStatics.PlaySound2D` "/Game/StarterContent/Audio/Explosion01.Explosion01" 1.0 1.0 0.0 null null)
      (if (not (`self.WinMenu?`))
        (set `self.WinMenu?` true)
        (bind _returnvalue_2 (`|CreateWidget` "/Game/Level/Win/WBP_Win3.WBP_Win3_C" _returnvalue))
        (bind _output_get (set `self.Winmenu3` _returnvalue_2))
        (`UserWidget.AddToViewport` _output_get 0)
        (`WidgetBlueprintLibrary.SetInputMode_GameAndUIEx` _returnvalue null)
        (set `PlayerController.bShowMouseCursor` true (`GameplayStatics.GetPlayerController` 0))
        (`GameplayStatics.SetGamePaused` true)
        (else
          (set `self.WinMenu?` false)
          (`Widget.RemoveFromParent` (`self.Winmenu3`))
          (`GameplayStatics.SetGamePaused` false)
          (`WidgetBlueprintLibrary.SetInputMode_GameOnly` _returnvalue)
          (set `PlayerController.bShowMouseCursor` false (`GameplayStatics.GetPlayerController` 0)))))))

(fn `UserConstructionScript`)